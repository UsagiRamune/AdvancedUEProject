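; BP_Terminal is an interactable terminal that opens and closes a WB_Terminal screen widget for a nearby player.
; Overlaps on ActivationPoint track whether a BP_ThirdPersonCharacter is in range and store it as Player.
; Interact calls ToggleTerminal, which, while in range, uses a FlipFlop to alternate between creating and removing the widget.
; Both branches set the mouse cursor visible, so closing does not hide it, and leaving range does not close the widget.
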(event `self.ActivationPoint.OnComponentBeginOverlap`
  (params (OverlappedComponent :type "PrimitiveComponent Object Reference") (OtherActor :type "Actor Object Reference") (OtherComp :type "PrimitiveComponent Object Reference") (OtherBodyIndex :type Integer) (bFromSweep :type Boolean) (SweepResult :type "HitResult Structure (by ref)"))
  (bind _asbp_third_person_character (cast `/Game/ThirdPerson/Blueprints/BP_ThirdPersonCharacter` OtherActor))
  (set `self.isInRange` true)
  (set `self.Player` _asbp_third_person_character))

(event `self.ActivationPoint.OnComponentEndOverlap`
  (params (OverlappedComponent :type "PrimitiveComponent Object Reference") (OtherActor :type "Actor Object Reference") (OtherComp :type "PrimitiveComponent Object Reference") (OtherBodyIndex :type Integer))
  (cast `/Game/ThirdPerson/Blueprints/BP_ThirdPersonCharacter` OtherActor)
  (set `self.isInRange` false)
  (set `self.Player` null))

(event `ToggleTerminal`
  (if (`self.isInRange`)
    (`/Engine/EditorBlueprintResources/StandardMacros.FlipFlop`
      (:`A`
        (bind _returnvalue (`|CreateWidget` "/Game/ProjectAssets/UI/WB_Terminal.WB_Terminal_C"))
        (bind _output_get (set `self.TerminalWidget` _returnvalue))
        (`UserWidget.AddToViewport` _output_get 0)
        (set `PlayerController.bShowMouseCursor` true (`GameplayStatics.GetPlayerController` 0)))
      (:`B`
        (`Widget.RemoveFromParent` (`self.TerminalWidget`))
        (set `PlayerController.bShowMouseCursor` true (`GameplayStatics.GetPlayerController` 0))))))

(event `/Game/ProjectAssets/Blueprint/Interfaces/BPI_Interact.Interact`
  (`self.ToggleTerminal`))

(fn `UserConstructionScript`)